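; BP_GoomAnimTest is a test player character with Enhanced Input movement, camera look, wheel zoom, jump and a Mario-style cap throw.
; Fire spawns one BP_Cap, and hold time drives its CapState from flight through stop to return, with release forcing return.
; Overlapping the cap after flight destroys it and re-arms throwing, launching the character upward if it was stopped.
; Tick only counts and prints an invulnerability timer; an older timing branch is unwired.
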(event `self.ReceiveControllerChanged`
  (params (OldController :type "Controller Object Reference") (NewController :type "Controller Object Reference"))
  ; 컨트롤러 받아오는 파트
  (bind _asplayer_controller (cast `PlayerController` NewController))
  (`EnhancedInputSubsystemInterface.AddMappingContext` (pcsubsystem `EnhancedInputLocalPlayerSubsystem` _asplayer_controller) "/Game/KJY/Inputs/IMC_Context.IMC_Context" 0 (struct)))

(event `self.ReceiveBeginPlay`
  ; 컨트롤러 받아오는 파트
  ;; 구버전
)

(event `InputAxisKey|MouseWheelAxis`
  (params (AxisValue :type "Float (single-precision)"))
  ; 카메라 줌 - 마우스 휠
  (set `SpringArmComponent.TargetArmLength` (+ (* AxisValue -25.0) (`SpringArmComponent.TargetArmLength` (`self.SpringArm`))) (`self.SpringArm`)))

(event `EnhancedInput|/Game/KJY/Inputs/IA_Look`
  (params (ActionValue :type "Vector2D Structure") (ElapsedSeconds :type "Float (double-precision)") (TriggeredSeconds :type "Float (double-precision)") (InputAction :type "InputAction Object Reference" :default "/Game/KJY/Inputs/IA_Look.IA_Look"))
  ; 카메라 이동 - 마우스 움직임
  (:`Triggered`
    (`self.AddControllerYawInput` (* (/ ActionValue_X 10.0) (`self.CameraSpeed`)))
    (`self.AddControllerPitchInput` (* (/ ActionValue_Y 10.0) (`self.CameraSpeed`)))))

(event `EnhancedInput|/Game/KJY/Inputs/IA_WASD`
  (params (ActionValue :type "Vector Structure") (ElapsedSeconds :type "Float (double-precision)") (TriggeredSeconds :type "Float (double-precision)") (InputAction :type "InputAction Object Reference" :default "/Game/KJY/Inputs/IA_WASD.IA_WASD"))
  (bind (_returnvalue_roll _returnvalue_pitch _returnvalue_yaw) (`KismetMathLibrary.BreakRotator` (`self.GetControlRotation`)))
  (bind (_returnvalue_roll_2 _returnvalue_pitch_2 _returnvalue_yaw_2) (`KismetMathLibrary.BreakRotator` (`self.GetControlRotation`)))
  ; NEW 무브파트
  (:`Triggered`
    (`self.AddMovementInput` (`KismetMathLibrary.GetRightVector` (`KismetMathLibrary.MakeRotator` _returnvalue_roll_2 0.0 _returnvalue_yaw_2)) ActionValue_X)
    (`self.AddMovementInput` (`KismetMathLibrary.GetForwardVector` (`KismetMathLibrary.MakeRotator` 0.0 0.0 _returnvalue_yaw)) ActionValue_Y)))

(event `EnhancedInput|/Game/KJY/Inputs/IA_Jump`
  (params (ActionValue :type Boolean) (ElapsedSeconds :type "Float (double-precision)") (TriggeredSeconds :type "Float (double-precision)") (InputAction :type "InputAction Object Reference" :default "/Game/KJY/Inputs/IA_Jump.IA_Jump"))
  ; 점프
  (:`Started`
    (`self.Jump`)))

(event `EnhancedInput|/Game/KJY/Inputs/IA_Fire`
  (params (ActionValue :type Boolean) (ElapsedSeconds :type "Float (double-precision)") (TriggeredSeconds :type "Float (double-precision)") (InputAction :type "InputAction Object Reference" :default "/Game/KJY/Inputs/IA_Fire.IA_Fire"))
  ; 공격부분
  (:`Triggered`
    (if (`self.CapSpawnCheck`)
      ;; 딜레이 발생
      (if (>= (`self.TriggeredCount`) (`self.MinAirTime`))
        (`/Engine/EditorBlueprintResources/StandardMacros.IsValid` (`self.BP_CCap`)
          (:`Is Valid`
            (set `/Game/KJY/BluePrints/BP_Cap.CapState` "NewEnumerator1" (`self.BP_CCap`)))))
      (if (>= (`self.TriggeredCount`) (`self.MaxAirTime`))
        (set `/Game/KJY/BluePrints/BP_Cap.CapState` "NewEnumerator2" (`self.BP_CCap`))
        (set `self.TriggeredCount` (`self.MaxAirTime`))
        (else
          (set `self.TriggeredCount` (+ (`self.TriggeredCount`) (`GameplayStatics.GetWorldDeltaSeconds`)))))))
  (:`Started`
    (if (not (`self.CapSpawnCheck`))
      (set `self._FloatTime` 0.0)
      (bind _returnvalue (`|SpawnActorFromClass` "/Game/KJY/BluePrints/BP_Cap.BP_Cap_C" (`SceneComponent.K2_GetComponentToWorld` (`self.FirePosition`)) "Undefined" "MultiplyWithRoot" null null))
      (`/Engine/EditorBlueprintResources/StandardMacros.IsValid` _returnvalue
        (:`Is Valid`
          (bind _output_get (set `self.BP_CCap` _returnvalue))
          (set `self.CapSpawnCheck` true)
          (set `/Game/KJY/BluePrints/BP_Cap.CapState` "NewEnumerator0" _output_get)))))
  (:`Completed`
    (`/Engine/EditorBlueprintResources/StandardMacros.IsValid` (`self.BP_CCap`)
      (:`Is Valid`
        (set `self.TriggeredCount` (`self.MaxAirTime`))
        (set `/Game/KJY/BluePrints/BP_Cap.CapState` "NewEnumerator2" (`self.BP_CCap`))
        (set `self.TriggeredCount` 0.0)))))

(event `self.ReceiveActorBeginOverlap`
  (params (OtherActor :type "Actor Object Reference"))
  ; 모자/마리오 충돌
  (if (== OtherActor (`self.BP_CCap`))
    (`/Engine/EditorBlueprintResources/StandardMacros.IsValid` (`self.BP_CCap`)
      (:`Is Valid`
        (if (`|EnumInequality` (`/Game/KJY/BluePrints/BP_Cap.CapState` (`self.BP_CCap`)) "NewEnumerator0")
          (if (`|EnumEquality` (`/Game/KJY/BluePrints/BP_Cap.CapState` (`self.BP_CCap`)) "NewEnumerator1")
            (`self.LaunchCharacter` (`KismetMathLibrary.MakeVector` 0.0 0.0 (* (`CharacterMovementComponent.JumpZVelocity` (`self.CharacterMovement`)) 1.2))) ; 정지중인 모자와 충돌시 마리오 발사!
          )
          (`self.K2_DestroyActor` (`self.BP_CCap`))
          (set `self.CapSpawnCheck` false)
          (set `self.TriggeredCount` 0.0))))))

(event `self.ReceiveTick`
  (params (DeltaSeconds :type "Float (single-precision)"))
  (if (and (`self.CanDamaged`) (<= (`self.CountUnbeatableTime`) (`self.MaxUnbeatableTime`))) :!pinned true
    (bind _output_get (set `self.CountUnbeatableTime` (+ (`self.CountUnbeatableTime`) (`GameplayStatics.GetWorldDeltaSeconds`))))
    (`KismetSystemLibrary.PrintString` (`KismetStringLibrary.Conv_DoubleToString` _output_get))))

(fn `UserConstructionScript`)