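; BP_PowerMoon is the goal pickup that ends the game when Mario touches it.
; On overlap it turns Mario toward the camera with a yaw offset, plays his goal montage and switches input to UI only.
; A timeline then raises the moon from its starting location, and on finish pauses the game, shows the mouse cursor and reveals the HUD's end widget.
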(event `self.ReceiveBeginPlay`
  (set `self.Location` (`self.K2_GetActorLocation`)))

(event `self.ReceiveActorBeginOverlap`
  (params (OtherActor :type "Actor Object Reference"))
  (bind _returnvalue (`GameplayStatics.GetPlayerController` 0))
  (bind (_location_x _location_y _location_z) (`KismetMathLibrary.BreakVector` (`self.Location`)))
  (bind _asbp_mario (cast `/Game/KJY/BluePrints/BP_Mario` OtherActor))
  (bind _output_get (set `self.BP_Mario` _asbp_mario))
  (bind (_returnvalue_roll _returnvalue_pitch _returnvalue_yaw) (`KismetMathLibrary.BreakRotator` (`KismetMathLibrary.FindLookAtRotation` (`self.K2_GetActorLocation` _output_get) (`PlayerCameraManager.GetCameraLocation` (`PlayerController.PlayerCameraManager` (`GameplayStatics.GetPlayerController` 0))))))
  (`self.K2_SetActorRotation` _output_get (`KismetMathLibrary.MakeRotator` 0.0 0.0 (+ _returnvalue_yaw -80.0)) false)
  (`Character.PlayAnimMontage` _output_get "/Game/Resource/Mario/Anim/Montage/MT_MarioGoal.MT_MarioGoal" 1.0 "None")
  (`WidgetBlueprintLibrary.SetInputMode_UIOnlyEx` (`GameplayStatics.GetPlayerController` 0) null "DoNotLock" true)
  (bind (_direction _moonup) (`Timeline|Timeline`)
    (:`Update`
      (`self.K2_SetActorLocation` (`KismetMathLibrary.MakeVector` _location_x _location_y (+ _location_z (* _moonup (`self.Size`))))))
    (:`Finished`
      (`GameplayStatics.SetGamePaused` true)
      (set `PlayerController.bShowMouseCursor` true _returnvalue)
      (`WidgetBlueprintLibrary.SetInputMode_UIOnlyEx` _returnvalue null)
      (bind _asbp_hud (cast `/Game/KHH/BluePrints/BP_HUD` (`PlayerController.GetHUD` _returnvalue)))
      (`Widget.SetVisibility` (`/Game/KHH/BluePrints/BP_HUD.WBP_End` _asbp_hud) "Visible"))))

(fn `UserConstructionScript`)