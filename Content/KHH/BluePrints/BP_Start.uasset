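; BP_Start sets up the game's start screen UI when play begins.
; BeginPlay creates the GameStart, MainMenu and SceneChange widgets, stores each in a variable and adds all three to the viewport.
; GameStart stays visible and the mouse cursor is enabled, while MainMenu and SceneChange start hidden.
; The Blueprint holds no logic for switching between them.
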(event `self.ReceiveBeginPlay`
  (bind _returnvalue (`|CreateWidget` "/Game/KHH/UI/WBP_GameStart.WBP_GameStart_C"))
  (bind _output_get (set `self.WBP_GameStart` _returnvalue))
  (`UserWidget.AddToViewport` _output_get 0)
  (set `PlayerController.bShowMouseCursor` true (`GameplayStatics.GetPlayerController` 0))
  (bind _returnvalue_2 (`|CreateWidget` "/Game/KHH/UI/WBP_MainMenu.WBP_MainMenu_C"))
  (bind _output_get_2 (set `self.WBP_MainMenu` _returnvalue_2))
  (`UserWidget.AddToViewport` _output_get_2 0)
  (`Widget.SetVisibility` _output_get_2 "Hidden")
  (bind _returnvalue_3 (`|CreateWidget` "/Game/KHH/UI/WBP_SceneChange.WBP_SceneChange_C"))
  (bind _output_get_3 (set `self.WBP_SceneChange` _returnvalue_3))
  (`UserWidget.AddToViewport` _output_get_3 0)
  (`Widget.SetVisibility` _output_get_3 "Hidden"))

(fn `UserConstructionScript`)