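; Mario's thrown cap actor, which captures a Goomba by handing player control to it on overlap.
; Each tick it spins its mesh and moves by CapState: forward, stopped, or back toward the player.
; It copies MinForwardTime and TriggeredCount from BP_Mario, though this graph never changes state with them.
; Overlapping a BP_Goom destroys the player pawn and cap, then possesses that Goomba.
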(event `self.ReceiveBeginPlay`
  ; MinForwardTime(전진해야하는 최소 시간) 체크.
  ;  한번만 받으면 되니 Event Begin에서.
  (bind _asbp_mario (cast `/Game/KJY/BluePrints/BP_Mario` (`GameplayStatics.GetPlayerPawn` 0)))
  (set `self.MinForwardTime2` (`/Game/KJY/BluePrints/BP_Mario.MinForwardTime` _asbp_mario)))

(event `self.ReceiveTick`
  (params (DeltaSeconds :type "Float (single-precision)"))
  (`SceneComponent.K2_AddLocalRotation` (`self.CapCube`) (`KismetMathLibrary.MakeRotator` 0.0 0.0 (* (`GameplayStatics.GetWorldDeltaSeconds`) (`self.CapRotateSpeed`))) false false) ; 모자 회전회오리
  ; 트리거 누른 시간 체크
  (bind _asbp_mario (cast `/Game/KJY/BluePrints/BP_Mario` (`GameplayStatics.GetPlayerPawn` 0)))
  (set `self.TriggeredCount2` (`/Game/KJY/BluePrints/BP_Mario.TriggeredCount` _asbp_mario))
  ; Comment
  (switch `/Game/KJY/BluePrints/CapState` (`self.CapState`)
    (:`NewEnumerator0`
      ;; CapGo / 모자 정면 방향
      (set `self.CapVector` (`SceneComponent.GetForwardVector` (`self.CapForward`))))
    (:`NewEnumerator1`
      (set `self.CapVector` (0.0 0.0 0.0)))
    (:`NewEnumerator2`
      ;; 플레이어 방향
      (set `self.CapVector` (- (`self.K2_GetActorLocation` (`GameplayStatics.GetPlayerPawn` 0)) (`self.K2_GetActorLocation`)))))
  (`self.K2_SetActorLocation` (+ (`self.K2_GetActorLocation`) (* (`KismetMathLibrary.Normal` (`self.CapVector`)) (`self.CapMoveSpeed`) (`GameplayStatics.GetWorldDeltaSeconds`)))))

(event `self.ReceiveActorBeginOverlap`
  (params (OtherActor :type "Actor Object Reference"))
  ; 굼바 충돌체크
  (bind _asbp_goom (cast `/Game/KHH/BluePrints/BP_Goom` OtherActor))
  (if (== _asbp_goom OtherActor)
    (`self.K2_DestroyActor` (`GameplayStatics.GetPlayerPawn` 0))
    (`self.K2_DestroyActor`)
    (`Controller.Possess` (`GameplayStatics.GetPlayerController` 0) _asbp_goom)))

(fn `UserConstructionScript`)