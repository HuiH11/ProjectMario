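; BP_Money is a spinning coin pickup that destroys itself when collected and increments MoneyCount in BP_GameModeBase.
; Overlap accepts Mario or his BP_Cap while the player pawn is BP_Mario; otherwise any BP_Goom can collect it.
; Tick yaws the Box at MoneySpinSpeed.
; An author note warns that coins placed too low miss the cap and collide like speed bumps.
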(event `self.ReceiveActorBeginOverlap`
  (params (OtherActor :type "Actor Object Reference"))
  ; 재화가 모자 OR 마리오에 부딪히면 마리오 점수가 올라감
  (bind _asbp_mario (cast `/Game/KJY/BluePrints/BP_Mario` (`GameplayStatics.GetPlayerPawn` 0))
    (:`then`
      (if (== _asbp_mario OtherActor)
        (`self.K2_DestroyActor` :!label _label)
        (bind _asbp_game_mode_base (cast `/Game/KJY/BluePrints/BP_GameModeBase` (`GameplayStatics.GetGameMode`)))
        (set `/Game/KJY/BluePrints/BP_GameModeBase.MoneyCount` (+ (`/Game/KJY/BluePrints/BP_GameModeBase.MoneyCount` _asbp_game_mode_base) 1) _asbp_game_mode_base)
        (else
          (bind _asbp_cap (cast `/Game/KJY/BluePrints/BP_Cap` OtherActor))
          (if (== _asbp_cap OtherActor)
            (goto _label)))))
    (:`CastFailed`
      (bind _asbp_goom (cast `/Game/KHH/BluePrints/BP_Goom` OtherActor))
      (if (== _asbp_goom OtherActor)
        (goto _label)))))

(event `self.ReceiveTick`
  (params (DeltaSeconds :type "Float (single-precision)"))
  (`SceneComponent.K2_AddLocalRotation` (`self.Box`) (`KismetMathLibrary.MakeRotator` 0.0 0.0 (* (`GameplayStatics.GetWorldDeltaSeconds`) (`self.MoneySpinSpeed`))) false false) ; 모자 회전회오리
)

(fn `UserConstructionScript`)